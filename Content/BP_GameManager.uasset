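; Game manager Blueprint that handles level restart and pause toggling.
; Restart reopens the current level by name and restores game-only input.
; PauseGame flips the paused state, showing or removing a pause menu widget that is created on first use and reused afterward.
; It also switches the first player controller between game-only and game-and-UI input and toggles the mouse cursor.
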(event Custom|Restart
  ;[0.15 0.15 0.15 0.5] Reload level
  (bind _returnvalue (Game|GetCurrentLevelName true))
  (Game|OpenLevel(byName) (Utilities|String|StringToName _returnvalue))
  ;[0.15 0.15 0.15 0.5] Re enable inputs
  (Input|SetInputModeGameOnly (Game|GetPlayerController 0) false))

(event Custom|PauseGame
  (bind _returnvalue (Game|GetPlayerController 0))
  (bind _returnvalue_2 (Game|GetPlayerController 0))
  (if (Game|IsGamePaused)
    (Widget|RemovefromParent (Variables|Default|GetPauseMenu))
    (Game|SetGamePaused false)
    (Input|SetInputModeGameOnly _returnvalue false)
    (Variables|/Script/Engine.PlayerController|SetbShowMouseCursor _returnvalue false)
    (else
      (if (Utilities|IsValid (Variables|Default|GetPauseMenu))
        (UserInterface|Viewport|AddtoViewport (Variables|Default|GetPauseMenu) 0)
        (else
          (bind _returnvalue_3 (UserInterface|CreateWidget "/Game/UI/PauseMenu.PauseMenu_C"))
          (bind _output_get (Variables|Default|SetPauseMenu _returnvalue_3))
          (UserInterface|Viewport|AddtoViewport _output_get 0)))
      (Game|SetGamePaused true)
      (Input|SetInputModeGameandUI _returnvalue_2 0 "DoNotLock" true false)
      (Variables|/Script/Engine.PlayerController|SetbShowMouseCursor _returnvalue_2 true))))